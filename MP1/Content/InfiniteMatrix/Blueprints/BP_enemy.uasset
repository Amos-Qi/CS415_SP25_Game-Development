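; BP_enemy is a slime enemy that damages the player on contact and can be killed by projectiles.
; Box overlap triggers a camera shake and, for BP_Player, subtracts score and health, updates both widgets, destroys the enemy and shows restart once health is depleted.
; A BP_Projectile overlapping the slime component awards score through the projectile's PlayerRef and destroys the enemy.
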(event OnComponentBeginOverlap(Box)
  (params (OverlappedComponent :type Primitive%20Component%20Object%20Reference) (OtherActor :type Actor%20Object%20Reference) (OtherComp :type Primitive%20Component%20Object%20Reference) (OtherBodyIndex :type Integer) (bFromSweep :type Boolean) (SweepResult :type Hit%20Result%20Structure%20%28by%20ref%29))
  (Camera|PlayWorldCameraShake "/Game/InfiniteMatrix/Blueprints/BP_CameraShake.BP_CameraShake_C" (Transformation|GetActorLocation) 0.0 1.4e+03 1.0 true)
  (bind _asbp_player (Utilities|Casting|CastToBP_Player OtherActor))
  (Utilities|FlowControl|Sequence
    (:then_0
      (bind _output_get (Variables|/Game/InfiniteMatrix/Blueprints/BP_Player.BP_Player_C|SetScore _asbp_player (+ (Variables|/Game/InfiniteMatrix/Blueprints/BP_Player.BP_Player_C|GetScore _asbp_player) -30)))
      (Default|UpdateScore (Variables|/Game/InfiniteMatrix/Blueprints/BP_Player.BP_Player_C|GetScoreBar _asbp_player) _output_get))
    (:then_1
      (bind _output_get_2 (Variables|/Game/InfiniteMatrix/Blueprints/BP_Player.BP_Player_C|SetHealth _asbp_player (- (Variables|/Game/InfiniteMatrix/Blueprints/BP_Player.BP_Player_C|GetHealth _asbp_player) 25.0)))
      (Default|UpdateHealthBar (Variables|/Game/InfiniteMatrix/Blueprints/BP_Player.BP_Player_C|GetWB_HealthBar _asbp_player) _output_get_2)))
  (Actor|DestroyActor)
  (if (<= _output_get_2 0.0)
    (Variables|/Game/InfiniteMatrix/Blueprints/BP_Player.BP_Player_C|SetIs%20Dead _asbp_player true)
    (Default|DisplayRestart _asbp_player)))

(event OnComponentBeginOverlap(cute_enemy_slime)
  (params (OverlappedComponent :type Primitive%20Component%20Object%20Reference) (OtherActor :type Actor%20Object%20Reference) (OtherComp :type Primitive%20Component%20Object%20Reference) (OtherBodyIndex :type Integer) (bFromSweep :type Boolean) (SweepResult :type Hit%20Result%20Structure%20%28by%20ref%29))
  (bind _asbp_projectile (Utilities|Casting|CastToBP_Projectile OtherActor))
  (bind _output_get (Variables|/Game/InfiniteMatrix/Blueprints/BP_Player.BP_Player_C|SetScore (Variables|/Game/InfiniteMatrix/Blueprints/BP_Projectile.BP_Projectile_C|GetPlayer_ref _asbp_projectile) (+ (Variables|/Game/InfiniteMatrix/Blueprints/BP_Player.BP_Player_C|GetScore (Variables|/Game/InfiniteMatrix/Blueprints/BP_Projectile.BP_Projectile_C|GetPlayer_ref _asbp_projectile)) 30)))
  (Default|UpdateScore (Variables|/Game/InfiniteMatrix/Blueprints/BP_Player.BP_Player_C|GetScoreBar (Variables|/Game/InfiniteMatrix/Blueprints/BP_Projectile.BP_Projectile_C|GetPlayer_ref _asbp_projectile)) _output_get)
  (Actor|DestroyActor))

(event EventBeginPlay)

(event Collision|EventActorBeginOverlap
  (params (OtherActor :type Actor%20Object%20Reference)))

(event EventTick
  (params (DeltaSeconds :type Float%20%28single-precision%29)))

(fn ConstructionScript)